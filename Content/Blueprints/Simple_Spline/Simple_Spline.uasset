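; Spline placement Blueprint that builds either a continuous path or repeated meshes along an editable spline in the construction script.
; Path mode adds a deformed spline mesh per segment with configurable width, height and material.
; Instance mode creates one instanced mesh component per listed mesh, then places uniformly scaled, spline-aligned instances at fixed spacing.
; Meshes are picked randomly or cycled in order, though the cycle skips the last of multiple entries.
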(fn `Instance Meshes`
  (bind _splinemeshcomponents (`self.SplineMeshComponents`))
  (bind _mesh_uniform_scale (`self.Mesh Uniform Scale`))
  (for _array_element (`self.Spline Mesh`)
    (bind _returnvalue (`AddComponent|NODE_AddInstancedStaticMeshComponent-0`))
    (`StaticMeshComponent.SetStaticMesh` _returnvalue _array_element)
    (`KismetArrayLibrary.Array_Add` (`self.SplineMeshComponents`) _returnvalue))
  (for _index (range (+ (`KismetMathLibrary.FFloor` (/ (`SplineComponent.GetSplineLength` (`self.Spline`)) (`self.Distance Offset`))) 1))
    (if (`self.Randomize Order`)
      (bind _returnvalue_2 (* _index (`self.Distance Offset`)))
      (bind _returnvalue_3 (`KismetMathLibrary.MakeTransform` (`SplineComponent.GetLocationAtDistanceAlongSpline` (`self.Spline`) _returnvalue_2 "Local") (`SplineComponent.GetRotationAtDistanceAlongSpline` (`self.Spline`) _returnvalue_2 "Local") (`KismetMathLibrary.MakeVector` _mesh_uniform_scale _mesh_uniform_scale _mesh_uniform_scale)))
      (`InstancedStaticMeshComponent.AddInstance` (`KismetArrayLibrary.Array_Random` _splinemeshcomponents) _returnvalue_3 false)
      (else
        (`InstancedStaticMeshComponent.AddInstance` (`|GetArrayItem` _splinemeshcomponents (`self.i`)) _returnvalue_3 false)
        (set `self.i` (+ (`self.i`) 1))
        (if (>= (`self.i`) (- (`KismetArrayLibrary.Array_Length` (`self.SplineMeshComponents`)) 1))
          (set `self.i` 0))))))

(fn `Spline Path`
  (bind _spline_path_width (`self.Spline Path Width`))
  (for _index (range (+ (- (`SplineComponent.GetNumberOfSplinePoints` (`self.Spline`)) 2) 1))
    (bind _returnvalue (`AddComponent|NODE_AddSplineMeshComponent-3` :`bManualAttachment` true))
    (`SceneComponent.SetWorldScale3D` _returnvalue (`KismetMathLibrary.MakeVector` 1.0 1.0 (`self.Spline Path Height`)))
    (`SplineMeshComponent.SetStartScale` _returnvalue (`KismetMathLibrary.MakeVector2D` _spline_path_width 1.0) true)
    (`SplineMeshComponent.SetEndScale` _returnvalue (`KismetMathLibrary.MakeVector2D` _spline_path_width 1.0) true)
    (`PrimitiveComponent.SetMaterial` _returnvalue 0 (`self.Spline Material`))
    (bind (_location _tangent) (`SplineComponent.GetLocationAndTangentAtSplinePoint` (`self.Spline`) _index "Local"))
    (bind (_location_2 _tangent_2) (`SplineComponent.GetLocationAndTangentAtSplinePoint` (`self.Spline`) (+ _index 1) "Local"))
    (`SplineMeshComponent.SetStartAndEnd` _returnvalue _location _tangent _location_2 _tangent_2 true)
    (`SceneComponent.K2_AttachToComponent` _returnvalue (`self.Spline`) "None" "KeepRelative" "KeepRelative" "KeepRelative" true)))

(fn `UserConstructionScript`
  ;[1 0.2922 0.2683] Mode Switch Logic
  (if (`self.Instance Meshes Along Spline`)
    (`self.Instance Meshes`)
    (else
      (`self.Spline Path`))))